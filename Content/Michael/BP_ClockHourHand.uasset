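; BP_ClockHourHand is a pickup actor for a clock's hour hand that the player collects through interaction.
; On BeginPlay it caches the BP_FirstPerson player and binds its InteractableComponent's interact dispatcher to a pickup event.
; Pickup sets HasHourClockHand on the player and destroys the actor.
; The InterfaceToggleFocus event switches custom depth rendering on the static mesh to mark focus.
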(event Custom|PickupClockHandEvent
  (Variables|/Game/ThirdPerson/Blueprints/BP_FirstPerson.BP_FirstPerson_C|SetbHasHourClockHand (Variables|Default|GetPlayer%20Ref) true)
  (Actor|DestroyActor))

(event EventInterfaceToggleFocus
  (params (Focus :type Boolean))
  (Rendering|SetRenderCustomDepth (Variables|Default|GetStaticMesh) Focus))

(event Collision|EventActorBeginOverlap
  (params (OtherActor :type Actor%20Object%20Reference)))

(event EventTick
  (params (DeltaSeconds :type Float%20%28single-precision%29)))

(event EventBeginPlay
  (bind _returnvalue (Actor|GetActorOfClass "/Game/ThirdPerson/Blueprints/BP_FirstPerson.BP_FirstPerson_C"))
  (Variables|Default|SetPlayer%20Ref _returnvalue)
  (EventDispatchers|BindEventtoOnInteractDispatcher (Variables|Default|GetInteractableComponent) (delegate Custom|PickupClockHandEvent)))

(fn ConstructionScript)
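; BP_Loopmigrate is a setup actor that streams in the LOOP1 level at BeginPlay and links the player to its interaction manager.
; After the non-blocking load completes, it finds BP_FirstPerson and BP_InteractManager by class and assigns the manager to the player's InteractManager reference.
; Debug prints mark progress.
; Disconnected leftover nodes, including a search for BP_DoorBathroom by display name, never run.
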(event EventBeginPlay
  (Game|LoadStreamLevel(byName) "LOOP1" true)
  (Development|PrintString "Loaded complete")
  (bind _returnvalue (Actor|GetActorOfClass "/Game/ThirdPerson/Blueprints/BP_FirstPerson.BP_FirstPerson_C"))
  (Variables|Default|SetPlayerref _returnvalue)
  (Actor|GetActorOfClass "/Game/Alexander/BP_InteractManager.BP_InteractManager_C")
  (Development|PrintString "Found interactmanager")
  (bind _returnvalue_2 (Actor|GetActorOfClass "/Game/Alexander/BP_InteractManager.BP_InteractManager_C"))
  (Variables|/Game/ThirdPerson/Blueprints/BP_FirstPerson.BP_FirstPerson_C|SetInteractManager (Variables|Default|GetPlayerref) _returnvalue_2))

(fn ConstructionScript)
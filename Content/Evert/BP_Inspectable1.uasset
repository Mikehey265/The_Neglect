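; BP_Inspectable1 is an actor that registers itself as the first-person player's inspectable object when inspected.
; On BeginPlay it binds BeginInspect to its InteractableComponent's inspect dispatcher and caches the BP_FirstPerson reference.
; BeginInspect sets the player's InspectableObject through a class lookup of BP_Inspectable1 rather than self, so it assumes a single instance.
; Unconnected nodes for validating and clearing that reference never run.
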(event Custom|BeginInspect
  (bind _returnvalue (Actor|GetActorOfClass "BP_Inspectable1_C"))
  (Variables|/Script/GP3_Team2.GP3_Team2Character|SetInspectableObject (Variables|Default|GetPlayerRef) _returnvalue))

(event EventBeginPlay
  (EventDispatchers|BindEventtoOnInspectDispatcher (Variables|Default|GetInteractableComponent) (delegate Custom|BeginInspect))
  (bind _returnvalue (Actor|GetActorOfClass "/Game/ThirdPerson/Blueprints/BP_FirstPerson.BP_FirstPerson_C"))
  (Variables|Default|SetPlayerRef _returnvalue))

(event Collision|EventActorBeginOverlap
  (params (OtherActor :type Actor%20Object%20Reference)))

(event EventTick
  (params (DeltaSeconds :type Float%20%28single-precision%29)))

(fn ConstructionScript)
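; BP_InfiniteHallway1 is a hallway segment that chains with BP_InfiniteHallway2 to create an infinite hallway effect.
; BeginPlay caches the player's BP_FirstPerson character, which both trigger volumes check on overlap.
; Loop3Trigger spawns a BP_InfiniteHallway2 at the attachment point, and Loop4Trigger destroys this segment.
; Disconnected leftover nodes hold an earlier spawn, previous-corridor cleanup and timeline-driven movement, none of which runs.
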(event OnComponentBeginOverlap(Loop3Trigger)
  (params (OverlappedComponent :type Primitive%20Component%20Object%20Reference) (OtherActor :type Actor%20Object%20Reference) (OtherComp :type Primitive%20Component%20Object%20Reference) (OtherBodyIndex :type Integer) (bFromSweep :type Boolean) (SweepResult :type Hit%20Result%20Structure%20%28by%20ref%29))
  (if (== OtherActor (Variables|Default|GetFirstPersonCharacter))
    (Game|SpawnActorfromClass "/Game/Kamil/Blueprints/InfinteHallway/BP_InfiniteHallway2.BP_InfiniteHallway2_C" (Transformation|GetWorldTransform (Variables|Default|GetAttachmentPoınt)) "Undefined" "MultiplyWithRoot" 0 (Game|GetPlayerCharacter 0))))

(event OnComponentBeginOverlap(Loop4Trigger)
  (params (OverlappedComponent :type Primitive%20Component%20Object%20Reference) (OtherActor :type Actor%20Object%20Reference) (OtherComp :type Primitive%20Component%20Object%20Reference) (OtherBodyIndex :type Integer) (bFromSweep :type Boolean) (SweepResult :type Hit%20Result%20Structure%20%28by%20ref%29))
  (if (== OtherActor (Variables|Default|GetFirstPersonCharacter))
    (Actor|DestroyActor)))

(event EventBeginPlay
  (bind _asbp_first_person (Utilities|Casting|CastToBP_FirstPerson (Game|GetPlayerCharacter 0)))
  (Variables|Default|SetFirstPersonCharacter _asbp_first_person))

(event Collision|EventActorBeginOverlap
  (params (OtherActor :type Actor%20Object%20Reference)))

(event EventTick
  (params (DeltaSeconds :type Float%20%28single-precision%29)))

(fn ConstructionScript)
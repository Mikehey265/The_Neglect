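; BP_PickableFlashlight is a flashlight actor with a toggleable SpotLight and a collision Box.
; The FlashLightOn/Off event uses a FlipFlop to play a 2D sound, then show or hide the light after a short delay.
; The Box overlap event is empty.
; Disconnected pickup logic, which would add a spotlight component to BP_FirstPerson and destroy the actor, never runs.
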(event OnComponentBeginOverlap(Box)
  (params (OverlappedComponent :type Primitive%20Component%20Object%20Reference) (OtherActor :type Actor%20Object%20Reference) (OtherComp :type Primitive%20Component%20Object%20Reference) (OtherBodyIndex :type Integer) (bFromSweep :type Boolean) (SweepResult :type Hit%20Result%20Structure%20%28by%20ref%29)))

(event Custom|FlashLightOn/Off
  (Utilities|FlowControl|FlipFlop
    (:A
      ;[0 0.4148 0.4479] Turn on/off sound
      (Audio|PlaySound2D 0 1.0 1.0 0.0 0 0)
      (Utilities|FlowControl|Delay 0.2)
      (Rendering|SetVisibility (Variables|Default|GetSpotLight) true false))
    (:B
      (Audio|PlaySound2D 0 1.0 1.0 0.0 0 0)
      (Utilities|FlowControl|Delay 0.2)
      (Rendering|SetVisibility (Variables|Default|GetSpotLight) false false))))

(fn ConstructionScript)
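; BP_InteractManager handles player interaction with whatever lies at the screen center.
; On BeginPlay it adds a cursor widget to the viewport and creates, but does not display, a keyhole widget.
; Each Tick it line-traces from the deprojected screen center out to InteractRange, showing the interact cursor when the hit actor has an InteractableComponent.
; Left click reuses that trace result and calls OnInteract on the component.
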(event Custom|OnLeftClick
  (if (Utilities|IsValid (Actor|GetComponentbyClass (.HitActor (Collision|BreakHitResult (stale EventTick _outhit))) "/Game/Alexander/InteractableComponent.InteractableComponent_C"))
    (Default|OnInteract (Actor|GetComponentbyClass (.HitActor (Collision|BreakHitResult (stale EventTick _outhit))) "/Game/Alexander/InteractableComponent.InteractableComponent_C"))))

(event EventBeginPlay
  (bind _returnvalue (UserInterface|CreateWidget "/Game/Alexander/WB_CursorUI.WB_CursorUI_C"))
  (bind _output_get (Variables|Default|SetCursorRef _returnvalue))
  (UserInterface|Viewport|AddtoViewport _output_get 0)
  (bind _returnvalue_2 (UserInterface|CreateWidget "/Game/Alexander/WB_KeyholeUI.WB_KeyholeUI_C"))
  (Variables|Default|SetKeyholeUI _returnvalue_2))

(event EventTick
  (params (DeltaSeconds :type Float%20%28single-precision%29))
  (bind _returnvalue (Game|GetPlayerController 0))
  (bind _returnvalue_2 (Viewport|GetViewportSize))
  (bind _cursorref (Variables|Default|GetCursorRef))
  (bind _returnvalue_3 (/ _returnvalue_2 "(X=2.000000,Y=2.000000)"))
  (bind _oninteractcursor (Variables|/Game/Alexander/WB_CursorUI.WB_CursorUI_C|GetOnInteractCursor _cursorref))
  (bind (_worldposition _worlddirection) (Class|GameplayStatics|DeprojectScreentoWorld _returnvalue _returnvalue_3))
  (bind (_outhit _returnvalue_4) (Collision|LineTraceByChannel _worldposition (+ _worldposition (* _worlddirection (Variables|Default|GetInteractRange))) "TraceTypeQuery1" false 0 "None"))
  (if _returnvalue_4
    (if (Utilities|IsValid (Actor|GetComponentbyClass (.HitActor (Collision|BreakHitResult _outhit)) "/Game/Alexander/InteractableComponent.InteractableComponent_C"))
      (Widget|SetVisibility _oninteractcursor "Visible")
      (else
        (Widget|SetVisibility _oninteractcursor "Hidden" :!label _label)))
    (else
      (goto _label))))

(fn ConstructionScript)
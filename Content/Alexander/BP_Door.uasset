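; BP_Door is an interactable door that swings open, partially open or closed, reports being locked, or offers a keyhole view.
; An InteractableComponent dispatcher runs a switch on DoorInteractState, setting the yaw target and next state.
; Tick eases the door toward that target with FInterpTo once rotation starts, and never clears the flag.
; The keyhole state temporarily moves the player camera, disables input and shows BP_InteractManager's keyhole UI before restoring them.
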(event Custom|BeginInteractLogic
  (bind _playerref (Variables|Default|GetPlayerRef))
  (bind _firstpersoncamera (Variables|/Script/GP3_Team2.GP3_Team2Character|GetFirstPersonCamera _playerref))
  (Development|PrintString "Door interact logic activated")
  (switch Utilities|FlowControl|Switch|SwitchonE_DoorInteractState (Variables|Default|GetDoorInteractState)
    (:NewEnumerator0
      (Development|PrintString "Door is opened")
      (Variables|Default|SetIsRotating true)
      (Variables|Default|SetRotationTarget 9e+01)
      (Variables|Default|SetDoorInteractState "NewEnumerator1"))
    (:NewEnumerator1
      (Development|PrintString "Door is closed")
      (Variables|Default|SetIsRotating true)
      (Variables|Default|SetRotationTarget 0.0)
      (Variables|Default|SetDoorInteractState "NewEnumerator1"))
    (:NewEnumerator2
      (Development|PrintString "Door is locked"))
    (:NewEnumerator3
      (Development|PrintString "partially open")
      (Variables|Default|SetIsRotating true)
      (Variables|Default|SetRotationTarget 25.0)
      (Variables|Default|SetDoorInteractState "NewEnumerator0"))
    (:NewEnumerator4
      (Development|PrintString "Lookthroughkeyhole")
      (bind _returnvalue (Actor|GetActorOfClass "/Game/Alexander/BP_InteractManager.BP_InteractManager_C"))
      (Variables|Default|SetInteractManager _returnvalue)
      (Variables|Default|SetCameraTransform (Transformation|GetWorldTransform _firstpersoncamera))
      (Transformation|SetWorldLocation _firstpersoncamera (+ "100.000000,10.000000,77.500000" (Transformation|GetActorLocation (Components|GetOwner))) false false)
      (Transformation|SetWorldRotation _firstpersoncamera "0.000000,-90.000000,0.000000" false false)
      (Input|DisableInput (Variables|Default|GetPlayerRef) (Game|GetPlayerController 0))
      (UserInterface|Viewport|AddtoViewport (Variables|/Game/Alexander/BP_InteractManager.BP_InteractManager_C|GetKeyholeUI (Variables|Default|GetInteractManager)) 0)
      (Utilities|FlowControl|Delay 5.0)
      (Transformation|SetWorldTransform (Variables|/Script/GP3_Team2.GP3_Team2Character|GetFirstPersonCamera (Variables|Default|GetPlayerRef)) (Variables|Default|GetCameraTransform) false false)
      (Input|EnableInput (Variables|Default|GetPlayerRef) (Game|GetPlayerController 0))
      (Widget|RemovefromParent (Variables|/Game/Alexander/BP_InteractManager.BP_InteractManager_C|GetKeyholeUI (Variables|Default|GetInteractManager))))))

(event Custom|HandleRotation
  (params (SetRotation :type Float%20%28double-precision%29))
  (Transformation|SetRelativeRotation (Variables|Default|GetDoor) (Math|Rotator|MakeRotator 0.0 0.0 (Math|Interpolation|FInterpTo (.Yaw (Math|Rotator|BreakRotator (Variables|/Script/Engine.SceneComponent|GetRelativeRotation (Variables|Default|GetDoor)))) SetRotation (Utilities|Time|GetWorldDeltaSeconds) (Variables|Default|GetInterp%20Speed))) false false))

(event EventBeginPlay
  (bind _returnvalue (Actor|GetActorOfClass "/Game/ThirdPerson/Blueprints/BP_FirstPerson.BP_FirstPerson_C"))
  (Variables|Default|SetPlayerRef _returnvalue)
  (EventDispatchers|BindEventtoOnInteractDispatcher (Variables|Default|GetInteractableComponent) (delegate Custom|BeginInteractLogic)))

(event Collision|EventActorBeginOverlap
  (params (OtherActor :type Actor%20Object%20Reference)))

(event EventTick
  (params (DeltaSeconds :type Float%20%28single-precision%29))
  (if (Variables|Default|GetIsRotating)
    (CallFunction|HandleRotation (Variables|Default|GetRotationTarget))))

(fn ConstructionScript)